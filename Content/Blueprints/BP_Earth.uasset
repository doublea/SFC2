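; BP_Earth is an Earth actor whose material lighting follows the direction of a referenced light source.
; On BeginPlay it creates a dynamic instance of M_Earth and, if LightSource is valid, writes that actor's forward vector into the LightDirection parameter before applying the instance to the Earth component.
; The direction is set only once at startup, and without a valid LightSource the dynamic material is never applied.
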(event `self.ReceiveBeginPlay`
  (bind _lightsource (`self.LightSource`))
  (bind _returnvalue (`KismetMaterialLibrary.CreateDynamicMaterialInstance` "/Game/Materials/M_Earth.M_Earth"))
  (set `self.MaterialInstance` _returnvalue)
  (if (`KismetSystemLibrary.IsValid` _lightsource)
    (`MaterialInstanceDynamic.SetVectorParameterValue` (`self.MaterialInstance`) "LightDirection" (`KismetMathLibrary.Conv_VectorToLinearColor` (`KismetMathLibrary.Conv_RotatorToVector` (`self.K2_GetActorRotation` _lightsource))))
    (`PrimitiveComponent.SetMaterial` (`self.Earth`) 0 (`self.MaterialInstance`))))

(fn `UserConstructionScript`)