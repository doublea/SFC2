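; BP_Photon is a homing projectile that damages the actor it is seeking.
; The construction script turns on homing on its ProjectileMovement component; the target component is not assigned in these graphs.
; On overlap it ignores all actors except the homing target's owner, to which it applies point damage credited to SourceActor before destroying itself.
; The hit is built manually from the projectile's location and reversed velocity direction.
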(event `self.ReceiveActorBeginOverlap`
  (params (OtherActor :type "Actor Object Reference"))
  (bind _homingtargetcomponent (`ProjectileMovementComponent.HomingTargetComponent` (`self.ProjectileMovement`)))
  (bind _returnvalue (`ActorComponent.GetOwner` _homingtargetcomponent))
  (`/Engine/EditorBlueprintResources/StandardMacros.IsValid` _homingtargetcomponent
    (:`Is Valid`
      (if (== OtherActor _returnvalue)
        (`GameplayStatics.ApplyPointDamage` _returnvalue 1.0 (`KismetMathLibrary.NegateVector` (`KismetMathLibrary.Normal` (`self.GetVelocity` self))) (`GameplayStatics.MakeHitResult` true true 0.0 (0.0 0.0 0.0) (`self.K2_GetActorLocation` self) (0.0 0.0 1.0) (0.0 0.0 1.0) null _returnvalue) null (`self.SourceActor`) (`self.DamageType`))
        (`self.K2_DestroyActor`)))))

(fn `UserConstructionScript`
  (set `ProjectileMovementComponent.bIsHomingProjectile` true (`self.ProjectileMovement`)))